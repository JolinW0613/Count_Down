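; BP_Grid is a map tile actor that randomly populates its SpawnArea with monsters and an optional barrier on BeginPlay.
; It spawns one or two of each monster type, plus one BP_Barrier1 when AllowBarrier is set, as loop bounds are inclusive.
; A shared SpawnOneComponent picks random points on the area's horizontal center plane, retrying up to ten times because colliding spawns that cannot be adjusted fail.
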(event EventBeginPlay
  (Utilities|FlowControl|Sequence
    (:then_0
      (CallFunction|SpawnMonster1 (Math|Random|RandomIntegerinRange 0 1)))
    (:then_1
      (CallFunction|SpawnMonster2 (Math|Random|RandomIntegerinRange 0 1)))
    (:then_2
      (if (Variables|Default|GetAllowBarrier)
        (CallFunction|SpawnBarrier1)))))

(event Collision|EventActorBeginOverlap
  (params (OtherActor :type Actor%20Object%20Reference)))

(event EventTick
  (params (DeltaSeconds :type Float%20%28single-precision%29)))

(fn ConstructionScript)

(fn SpawnMonster1
  (params (NumOfMon1 :type Integer))
  (for _index (range 0 NumOfMon1) ; Born certain number of mon1 inside the model
    (CallFunction|SpawnOneComponent "/Game/BluePrint/BP_Monster1.BP_Monster1_C")))

(fn SpawnOneComponent
  (params (ComponentClass :type Actor%20Class%20Reference))
  (bind _spawn_area (Variables|Default|GetSpawn%20Area))
  (bind (_origin _boxextent) (Collision|GetComponentBounds _spawn_area))
  ;[0.15 0.15 0.15 0.5] Put new object to the map without overlapping on each other
  (Utilities|FlowControl|ForLoopwithBreak 0 9 :!label _label ; Try 10 random points; break when spawn succeeds
    (:LoopBody
      (bind _returnvalue (Game|SpawnActorfromClass ComponentClass (Math|Transform|MakeTransform (Math|Random|RandomPointinBoundingBox (Math|Vector|MakeVector (.x _origin) (.y _origin) (.z _origin)) (Math|Vector|MakeVector (.x _boxextent) (.y _boxextent) 0.0))) "AdjustIfPossibleButDontSpawnIfColliding" "MultiplyWithRoot" 0 0))
      (Utilities|IsValid _returnvalue
        (:Is%20Valid
          (goto _label Break))))))

(fn SpawnMonster2
  (params (Num%20OfMon2 :type Integer))
  (for _index (range 0 Num%20OfMon2) ; Born certain number of mon1 inside the model
    (CallFunction|SpawnOneComponent "/Game/BluePrint/BP_Monster2.BP_Monster2_C")))

(fn SpawnBarrier1
  (params (NumOfB1 :type Integer))
  (for _index (range 0 NumOfB1) ; Born certain number of mon1 inside the model
    (CallFunction|SpawnOneComponent "/Game/BluePrint/BP_Barrier1.BP_Barrier1_C")))