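; BP_MapGenerator builds a random map of connected BP_Grid tiles, with tile and monster counts scaled by GameDifficulty.
; It grows outward from random open tile arrows, tracking occupied locations and spacing barriers by cooldown and minimum distance.
; It shuffles a monster class list that RequestMonsterClass hands out sequentially until exhausted.
; The same generation runs on BeginPlay, marked for removal, and in GenerateMap.
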(event EventBeginPlay
  (bind _availablearrows (Variables|Default|GetAvailableArrows))
  ;[0.15 0.15 0.15 0.5] Random map generator (remove)
  (CallFunction|InitializeDifficulty)
  (CallFunction|BuildMonsterSpawnList)
  (bind _returnvalue (Game|SpawnActorfromClass "/Game/BluePrint/BP_Grid.BP_Grid_C" (Math|Conversions|ToTransform(Vector) (Transformation|GetActorLocation)) "AlwaysSpawn" "MultiplyWithRoot" 0 false 0))
  (Variables|Default|SetGridStep (* (.X (Math|Vector|BreakVector (.BoxExtent (Collision|GetComponentBounds (Variables|/Game/BluePrint/BP_Grid.BP_Grid_C|GetCube _returnvalue))))) 2.0))
  (Utilities|Array|Clear _availablearrows)
  (Utilities|Array|AppendArray _availablearrows (Utilities|Array|MakeArray (Variables|/Game/BluePrint/BP_Grid.BP_Grid_C|GetArrow0 _returnvalue) (Variables|/Game/BluePrint/BP_Grid.BP_Grid_C|GetArrow1 _returnvalue) (Variables|/Game/BluePrint/BP_Grid.BP_Grid_C|GetArrow2 _returnvalue) (Variables|/Game/BluePrint/BP_Grid.BP_Grid_C|GetArrow3 _returnvalue)))
  (bind _gridnum (CallFunction|GetGridNumberbyDifficulty))
  (for _index (range 0 _gridnum)
    (bind _output_get (Variables|Default|SetSelectedArrow (.OutItem (Utilities|Array|Random (Variables|Default|GetAvailableArrows)))))
    (Utilities|IsValid _output_get
      (:Is%20Valid
        (bind _output_get_2 (Variables|Default|SetCandidateLocation (+ (Transformation|GetWorldLocation (Variables|Default|GetSelectedArrow)) (* (Math|Vector|GetForwardVector (Variables|Default|GetSelectedArrow)) (/ (Variables|Default|GetGridStep) 2.0)))))
        (bind _return (CallFunction|IsBarrierTooClose (Variables|Default|GetCandidateLocation)))
        (bind _output_get_3 (Variables|Default|SetShouldSpawnBarrier (and (<= (Variables|Default|GetBarrierCooldown) 0) (not _return))))
        (if (not (Utilities|Array|ContainsItem (Variables|Default|GetOccupiedLocations) _output_get_2))
          (bind _returnvalue_2 (Game|SpawnActorfromClass "/Game/BluePrint/BP_Grid.BP_Grid_C" (Math|Transform|MakeTransform _output_get_2) "Undefined" "MultiplyWithRoot" 0 _output_get_3 0))
          (Utilities|Array|RemoveItem (Variables|Default|GetAvailableArrows) (Variables|Default|GetSelectedArrow))
          (Utilities|FlowControl|Sequence
            (:then_0
              (if (Variables|Default|GetShouldSpawnBarrier)
                (Variables|Default|SetBarrierCooldown 3)
                (else
                  (Variables|Default|SetBarrierCooldown (Math|Integer|Max(Integer) (- (Variables|Default|GetBarrierCooldown) 1))))))
            (:then_1
              (Utilities|Array|AddUnique (Variables|Default|GetOccupiedLocations) (Variables|Default|GetCandidateLocation))
              (Utilities|Array|AppendArray (Variables|Default|GetAvailableArrows) (Utilities|Array|MakeArray (Variables|/Game/BluePrint/BP_Grid.BP_Grid_C|GetArrow0 _returnvalue_2) (Variables|/Game/BluePrint/BP_Grid.BP_Grid_C|GetArrow1 _returnvalue_2) (Variables|/Game/BluePrint/BP_Grid.BP_Grid_C|GetArrow2 _returnvalue_2) (Variables|/Game/BluePrint/BP_Grid.BP_Grid_C|GetArrow3 _returnvalue_2)))
              (if (Variables|Default|GetShouldSpawnBarrier)
                (Utilities|Array|AddUnique (Variables|Default|GetBarrierLocations) (Variables|Default|GetCandidateLocation)))))))
      (:Is%20Not%20Valid
        (Development|PrintString "Falied to select arrow")))))

(event Collision|EventActorBeginOverlap
  (params (OtherActor :type Actor%20Object%20Reference)))

(event EventTick
  (params (DeltaSeconds :type Float%20%28single-precision%29)))

(fn ConstructionScript)

(fn IsBarrierTooClose
  (params (Location :type Vector))
  (LocalVariables|SetTooClose false)
  (bind _array_element (Utilities|Array|ForEachLoopwithBreak (Variables|Default|GetBarrierLocations) :!label _label)
    (:LoopBody
      (if (< (Math|Vector|Distance(Vector) _array_element Location) 1.5e+03)
        (LocalVariables|SetTooClose true)
        (goto _label Break)))
    (:Completed
      (return (LocalVariables|GetTooClose)))))

(fn InitializeDifficulty
  (switch Utilities|FlowControl|Switch|SwitchonE_GameDifficulty (Variables|Default|GetGameDifficulty)
    (:NewEnumerator0
      (Variables|Default|SetTargetMonster1Count 3)
      (Variables|Default|SetTargetMonster2Count 3)
      (Variables|Default|SetSpawnedMonster1Count 0)
      (Variables|Default|SetSpawnedMonster2Count 0))
    (:NewEnumerator1
      (Variables|Default|SetTargetMonster1Count 5)
      (Variables|Default|SetTargetMonster2Count 5)
      (Variables|Default|SetTargetMonster3Count 2)
      (Variables|Default|SetSpawnedMonster1Count 0)
      (Variables|Default|SetSpawnedMonster2Count 0)
      (Variables|Default|SetSpawnedMonster3Count 0))
    (:NewEnumerator2
      (Variables|Default|SetTargetMonster1Count 8)
      (Variables|Default|SetTargetMonster2Count 8)
      (Variables|Default|SetTargetMonster3Count 5)
      (Variables|Default|SetSpawnedMonster1Count 0)
      (Variables|Default|SetSpawnedMonster2Count 0)
      (Variables|Default|SetSpawnedMonster3Count 0))))

(fn RequestMonsterClass
  (if (< (Variables|Default|GetMonsterSpawnIndex) (Utilities|Array|Length (Variables|Default|GetMonsterSpawnList)))
    (bind _output_get (LocalVariables|SetRequestedMonsterClass (Utilities|Array|Get(acopy) (Variables|Default|GetMonsterSpawnList) (Variables|Default|GetMonsterSpawnIndex))))
    (Variables|Default|SetMonsterSpawnIndex (+ (Variables|Default|GetMonsterSpawnIndex) 1))
    (return true _output_get)
    (else
      (return false 0))))

(fn BuildMonsterSpawnList
  (Utilities|Array|Clear (Variables|Default|GetMonsterSpawnList))
  (Variables|Default|SetMonsterSpawnIndex 0)
  (for _index (range 0 (- (Variables|Default|GetTargetMonster1Count) 1))
    (Utilities|Array|Add (Variables|Default|GetMonsterSpawnList) "/Game/BluePrint/BP_Monster1.BP_Monster1_C"))
  (for _index_2 (range 0 (- (Variables|Default|GetTargetMonster2Count) 1))
    (Utilities|Array|Add (Variables|Default|GetMonsterSpawnList) "/Game/BluePrint/BP_Monster2.BP_Monster2_C"))
  (for _index_3 (range 0 (- (Variables|Default|GetTargetMonster3Count) 1))
    (Utilities|Array|Add (Variables|Default|GetMonsterSpawnList) "/Game/BluePrint/BP_Monster3.BP_Monster3_C"))
  (Utilities|Array|Shuffle (Variables|Default|GetMonsterSpawnList)))

(fn GetGridNumberbyDifficulty
  (switch Utilities|FlowControl|Switch|SwitchonE_GameDifficulty (Variables|Default|GetGameDifficulty)
    (:NewEnumerator0
      (return 9))
    (:NewEnumerator1
      (return 21))
    (:NewEnumerator2
      (return 41))))

(fn GenerateMap
  (bind _availablearrows (Variables|Default|GetAvailableArrows))
  ;[0.15 0.15 0.15 0.5] Random map generator
  (CallFunction|InitializeDifficulty)
  (CallFunction|BuildMonsterSpawnList)
  (bind _returnvalue (Game|SpawnActorfromClass "/Game/BluePrint/BP_Grid.BP_Grid_C" (Math|Conversions|ToTransform(Vector) (Transformation|GetActorLocation)) "AlwaysSpawn" "MultiplyWithRoot" 0 false 0))
  (Variables|Default|SetGridStep (* (.X (Math|Vector|BreakVector (.BoxExtent (Collision|GetComponentBounds (Variables|/Game/BluePrint/BP_Grid.BP_Grid_C|GetCube _returnvalue))))) 2.0))
  (Utilities|Array|Clear _availablearrows)
  (Utilities|Array|AppendArray _availablearrows (Utilities|Array|MakeArray (Variables|/Game/BluePrint/BP_Grid.BP_Grid_C|GetArrow0 _returnvalue) (Variables|/Game/BluePrint/BP_Grid.BP_Grid_C|GetArrow1 _returnvalue) (Variables|/Game/BluePrint/BP_Grid.BP_Grid_C|GetArrow2 _returnvalue) (Variables|/Game/BluePrint/BP_Grid.BP_Grid_C|GetArrow3 _returnvalue)))
  (bind _gridnum (CallFunction|GetGridNumberbyDifficulty))
  (for _index (range 0 _gridnum)
    (bind _output_get (Variables|Default|SetSelectedArrow (.OutItem (Utilities|Array|Random (Variables|Default|GetAvailableArrows)))))
    (Utilities|IsValid _output_get
      (:Is%20Valid
        (bind _output_get_2 (Variables|Default|SetCandidateLocation (+ (Transformation|GetWorldLocation (Variables|Default|GetSelectedArrow)) (* (Math|Vector|GetForwardVector (Variables|Default|GetSelectedArrow)) (/ (Variables|Default|GetGridStep) 2.0)))))
        (bind _return (CallFunction|IsBarrierTooClose (Variables|Default|GetCandidateLocation)))
        (bind _output_get_3 (Variables|Default|SetShouldSpawnBarrier (and (<= (Variables|Default|GetBarrierCooldown) 0) (not _return))))
        (if (not (Utilities|Array|ContainsItem (Variables|Default|GetOccupiedLocations) _output_get_2))
          (bind _returnvalue_2 (Game|SpawnActorfromClass "/Game/BluePrint/BP_Grid.BP_Grid_C" (Math|Transform|MakeTransform _output_get_2) "Undefined" "MultiplyWithRoot" 0 _output_get_3 0))
          (Utilities|Array|RemoveItem (Variables|Default|GetAvailableArrows) (Variables|Default|GetSelectedArrow))
          (Utilities|FlowControl|Sequence
            (:then_0
              (if (Variables|Default|GetShouldSpawnBarrier)
                (Variables|Default|SetBarrierCooldown 3)
                (else
                  (Variables|Default|SetBarrierCooldown (Math|Integer|Max(Integer) (- (Variables|Default|GetBarrierCooldown) 1))))))
            (:then_1
              (Utilities|Array|AddUnique (Variables|Default|GetOccupiedLocations) (Variables|Default|GetCandidateLocation))
              (Utilities|Array|AppendArray (Variables|Default|GetAvailableArrows) (Utilities|Array|MakeArray (Variables|/Game/BluePrint/BP_Grid.BP_Grid_C|GetArrow0 _returnvalue_2) (Variables|/Game/BluePrint/BP_Grid.BP_Grid_C|GetArrow1 _returnvalue_2) (Variables|/Game/BluePrint/BP_Grid.BP_Grid_C|GetArrow2 _returnvalue_2) (Variables|/Game/BluePrint/BP_Grid.BP_Grid_C|GetArrow3 _returnvalue_2)))
              (if (Variables|Default|GetShouldSpawnBarrier)
                (Utilities|Array|AddUnique (Variables|Default|GetBarrierLocations) (Variables|Default|GetCandidateLocation)))))))
      (:Is%20Not%20Valid
        (Development|PrintString "Falied to select arrow")))))