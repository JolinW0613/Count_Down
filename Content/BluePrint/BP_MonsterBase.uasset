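; Base AI monster character with health, trait-based attacks and ragdoll death.
; TryAttack uses MonsterTraits to pick melee damage, a spawned projectile or a proximity self-destruct; BeginPlay calls it once on the player, then snaps to navmesh.
; Fire separately line-traces toward the AI focus actor with random spread.
; AnyDamage lowers HP, swaps materials and reports to AI damage sensing; at zero it unpossesses, ragdolls and sets a lifespan.
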(event Custom|Fire
  (bind _self self)
  (bind _returnvalue (AI|GetAIController _self))
  (bind _returnvalue_2 (Class|AIController|GetFocusActor _returnvalue))
  ;[0.15 0.15 0.15 0.5] Shoot the bullet once
  (Utilities|IsValid _returnvalue_2
    (:Is%20Valid
      (bind _outhit (Collision|LineTraceByChannel (Transformation|GetWorldLocation (Variables|Default|GetGun%28Needs%20to%20be%20changed%29)) (Math|Vector|RotateVector (Transformation|GetActorLocation _returnvalue_2) (Math|Rotator|MakeRotator (Math|Random|RandomFloatinRange -1.0 1.0) (Math|Random|RandomFloatinRange -1.0 1.0) (Math|Random|RandomFloatinRange -1.0 1.0))) "TraceTypeQuery1" false 0 "None"))
      (Game|Damage|ApplyPointDamage (.HitActor (Collision|BreakHitResult _outhit)) 0.0 (.ImpactNormal (Collision|BreakHitResult _outhit)) _outhit 0 self)
      (Niagara|SpawnSystematLocation 0 (.TraceStart (Collision|BreakHitResult _outhit)) (Math|Rotator|FindLookatRotation (.TraceStart (Collision|BreakHitResult _outhit)) (.TraceEnd (Collision|BreakHitResult _outhit))))
      (Audio|PlaySoundatLocation "/Engine/VREditor/Sounds/UI/Camera_Shutter.Camera_Shutter" (Transformation|GetActorLocation) "0, 0, 0" 1.0 1.0 0.0 0 0 0 0))))

(event Custom|EnemyDeath
  (bind _self self)
  (bind _mesh (Variables|Character|GetMesh))
  (bind _returnvalue (AI|GetAIController _self))
  ;[0.15 0.15 0.15 0.5] Able to get the gun after enemy death
  (Utilities|IsValid _returnvalue
    (:Is%20Valid
      (Pawn|UnPossess _returnvalue))
    (:Is%20Not%20Valid
      _))
  (Collision|SetCollisionEnabled _mesh "PhysicsOnly")
  (Physics|SetSimulatePhysics _mesh true)
  (Collision|SetCollisionEnabled (Variables|Collision|GetCapsuleComponent) "NoCollision")
  (Actor|SetLifeSpan 5.0))

(event EventBeginPlay
  (bind _returnvalue (Transformation|GetActorLocation))
  (bind _mesh (Variables|Character|GetMesh))
  (bind (_projectedlocation _returnvalue_2) (AI|Navigation|ProjectPointtoNavigation _returnvalue 0 0 "150.000000,150.000000,500.000000"))
  (Utilities|FlowControl|Sequence
    (:then_0
      (Transformation|SetRelativeLocationAndRotation (Variables|Default|GetGun%28Needs%20to%20be%20changed%29) (Transformation|GetWorldLocation _mesh) (Transformation|GetWorldRotation _mesh) false false))
    (:then_1
      (CallFunction|TryAttack (Game|GetPlayerCharacter 0))
      (Utilities|FlowControl|Delay 0.5)
      (if _returnvalue_2
        (Transformation|SetActorLocation _projectedlocation false false)
        (else
          (Development|PrintString "NAV PROJECTION FAILED"))))
    (:then_2
      (Variables|Default|SetCurrentHP (Variables|Default|GetMaxHP)))))

(event Game|Damage|EventAnyDamage
  (params (Damage :type Float%20%28single-precision%29) (DamageType :type Damage%20Type%20Object%20Reference) (InstigatedBy :type Controller%20Object%20Reference) (DamageCauser :type Actor%20Object%20Reference))
  (bind _returnvalue (Transformation|GetActorLocation))
  (bind _mesh (Variables|Character|GetMesh))
  ;[0.15 0.15 0.15 0.5] Check death state of monsters
  (bind _output_get (Variables|Default|SetCurrentHP (Math|Float|Clamp(Float) (- (Variables|Default|GetCurrentHP) Damage) 0.0 (Variables|Default|GetMaxHP))))
  (if (<= _output_get 0.0)
    (CallFunction|EnemyDeath)
    (else
      (Rendering|Material|SetMaterial _mesh 0 0)
      (Utilities|FlowControl|Delay 0.5)
      (Rendering|Material|SetMaterial _mesh 0 0)
      (Audio|PlaySoundatLocation "/Engine/VREditor/Sounds/UI/Camera_Shutter.Camera_Shutter" _returnvalue "0, 0, 0" 1.0 1.0 0.0 0 0 0 0)
      (if (<= _output_get 0.0)
        (CallFunction|EnemyDeath)
        (Utilities|FlowControl|Delay 0.1)
        (Components|DestroyComponent (Variables|Character|GetMesh))
        (Development|PrintString "111")
        (else
          (Class|AISenseDamage|ReportDamageEvent self DamageCauser 1e+01 _returnvalue "0, 0, 0" "None"))))))

(fn ConstructionScript)

(fn HasTraits
  (params (Trait :type E_MonsterTrait%20Enum :default "NewEnumerator0"))
  ;[0.15 0.15 0.15 0.5] Check wheather a monster has a certain trait
  (return (Utilities|Set|Contains (Variables|Default|GetMonsterTraits) Trait)))

(fn TryAttack
  (params (TargetActor :type Actor%20Object%20Reference))
  (if (Variables|Default|GetCanAttack)
    (Development|PrintString "Attack Success")
    (bind _hastrait (CallFunction|HasTraits "NewEnumerator1"))
    (if _hastrait
      (CallFunction|MeleeAttack TargetActor)
      (else
        (bind _hastrait_2 (CallFunction|HasTraits "NewEnumerator0"))
        (if _hastrait_2
          (CallFunction|RangedAttack TargetActor)
          (else
            (CallFunction|HasTraits "NewEnumerator2")
            (CallFunction|SelfDestructAttack TargetActor)))))
    (else
      (Development|PrintString "Can't Attack"))))

(fn MeleeAttack
  (params (TargetActor :type Actor%20Object%20Reference))
  ;[0.15 0.15 0.15 0.5] Cause a frame of Melee Attack
  (Utilities|IsValid TargetActor
    (:Is%20Valid
      (Game|Damage|ApplyDamage TargetActor (Variables|Default|GetMeleeDamage) (Pawn|GetController) self))))

(fn RangedAttack
  (params (TargetActor :type Actor%20Object%20Reference))
  (bind _self self)
  (bind _projectilespawnpoint (Variables|Default|GetProjectileSpawnPoint))
  (bind _returnvalue (Transformation|GetWorldLocation _projectilespawnpoint))
  (Utilities|IsValid TargetActor
    (:Is%20Valid
      (Game|SpawnActorfromClass (Variables|Default|GetStickerClass) (Math|Transform|MakeTransform _returnvalue (Math|Rotator|FindLookatRotation _returnvalue (Transformation|GetActorLocation TargetActor))) "AdjustIfPossibleButAlwaysSpawn" "MultiplyWithRoot" _self _self))))

(fn SelfDestructAttack
  (params (TargetActor :type Actor%20Object%20Reference))
  (bind _self self)
  (Utilities|IsValid TargetActor
    (:Is%20Valid
      (if (<= (Transformation|GetDistanceTo self TargetActor) (Variables|Default|GetExplosionTriggerDistance))
        (Game|Damage|ApplyRadialDamage (Variables|Default|GetExplosionDamage) (Transformation|GetActorLocation _self) (Variables|Default|GetExplosionRadius) 0 0 self (Pawn|GetController _self) true "ECC_Visibility")
        (Actor|DestroyActor)))))