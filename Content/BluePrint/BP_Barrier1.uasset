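; BP_Barrier1 is a physics-driven barrier that knocks the twin-stick player character away when the two collide.
; Its Box component starts simulating physics on BeginPlay.
; On a hit with BP_TwinStickCharacter, it launches the character horizontally away from the barrier's location with a small upward boost.
; The launch overrides horizontal velocity but adds to the existing vertical velocity.
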(event OnComponentHit(Box)
  (params (HitComponent :type Primitive%20Component%20Object%20Reference) (OtherActor :type Actor%20Object%20Reference) (OtherComp :type Primitive%20Component%20Object%20Reference) (NormalImpulse :type Vector :default "0, 0, 0") (Hit :type Hit%20Result%20Structure%20%28by%20ref%29))
  (bind _asbp_twin_stick_character (Utilities|Casting|CastToBP_TwinStickCharacter OtherActor))
  (Character|LaunchCharacter _asbp_twin_stick_character (Math|Vector|MakeVector (.X (Math|Vector|BreakVector (* (Class|KismetMathLibrary|VectorNormal2D (- (Transformation|GetActorLocation _asbp_twin_stick_character) (Transformation|GetActorLocation self)) 0.0001) 5e+02))) (.Y (Math|Vector|BreakVector (* (Class|KismetMathLibrary|VectorNormal2D (- (Transformation|GetActorLocation _asbp_twin_stick_character) (Transformation|GetActorLocation self)) 0.0001) 5e+02))) 1.5e+02) true false))

(event EventBeginPlay
  (Physics|SetSimulatePhysics (Variables|Default|GetBox) true))

(fn ConstructionScript)