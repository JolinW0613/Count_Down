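; BP_MonsterNormalBullet is a monster bullet that damages the twin-stick player character on contact.
; It runs its parent's BeginPlay, then limits its own lifespan to a few seconds.
; Collision overlaps are filtered to BP_TwinStickCharacter actors other than the owner.
; A DoOnce gate lets only the first valid hit apply damage, credited to the instigator's controller, before the bullet destroys itself.
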(event OnComponentBeginOverlap(Collision)
  (params (OverlappedComponent :type Primitive%20Component%20Object%20Reference) (OtherActor :type Actor%20Object%20Reference) (OtherComp :type Primitive%20Component%20Object%20Reference) (OtherBodyIndex :type Integer) (bFromSweep :type Boolean) (SweepResult :type Hit%20Result%20Structure%20%28by%20ref%29))
  (Utilities|IsValid OtherActor
    (:Is%20Valid
      (bind _asbp_twin_stick_character (Utilities|Casting|CastToBP_TwinStickCharacter OtherActor))
      (if (!= OtherActor (Components|GetOwner))
        (Utilities|FlowControl|DoOnce false
          (:Completed
            (Game|Damage|ApplyDamage _asbp_twin_stick_character (Variables|Default|GetBulletDamage) (Game|GetInstigatorController) self "/Script/Engine.DamageType")
            (Actor|DestroyActor)))))))

(event EventBeginPlay
  (|CallParentFunction)
  (Actor|SetLifeSpan 5.0))

(fn ConstructionScript)