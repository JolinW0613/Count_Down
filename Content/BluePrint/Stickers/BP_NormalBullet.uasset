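; BP_NormalBullet is a bullet that damages monsters it overlaps and expires five seconds after spawning.
; Its Collision overlap casts the other actor to BP_MonsterBase, then passes a DoOnce to apply BulletDamage and destroy the bullet.
; The owner check compares the hit actor with that actor's own owner, and the damage instigator also comes from the hit actor.
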(event OnComponentBeginOverlap(Collision)
  (params (OverlappedComponent :type Primitive%20Component%20Object%20Reference) (OtherActor :type Actor%20Object%20Reference) (OtherComp :type Primitive%20Component%20Object%20Reference) (OtherBodyIndex :type Integer) (bFromSweep :type Boolean) (SweepResult :type Hit%20Result%20Structure%20%28by%20ref%29))
  (Utilities|IsValid OtherActor
    (:Is%20Valid
      (bind _asbp_monster_base (Utilities|Casting|CastToBP_MonsterBase OtherActor))
      (Utilities|IsValid _asbp_monster_base
        (:Is%20Valid
          (if (!= OtherActor (Components|GetOwner OtherActor))
            (Utilities|FlowControl|DoOnce false
              (:Completed
                (Game|Damage|ApplyDamage _asbp_monster_base (Variables|Default|GetBulletDamage) (Game|GetInstigatorController OtherActor) self "/Script/Engine.DamageType")
                (Actor|DestroyActor)))))))))

(event EventBeginPlay
  (|CallParentFunction)
  (Actor|SetLifeSpan 5.0))

(fn ConstructionScript)