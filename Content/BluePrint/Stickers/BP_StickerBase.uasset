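; BP_StickerBase is a sticker projectile, named as a base class, that damages the first actor it overlaps other than its owner.
; On BeginPlay it sets a three-second lifespan, although the graph comment says two.
; Collision overlaps feed HandleImpact, which applies Damage credited to the instigator's controller and then destroys the sticker.
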(event OnComponentBeginOverlap(Collision)
  (params (OverlappedComponent :type Primitive%20Component%20Object%20Reference) (OtherActor :type Actor%20Object%20Reference) (OtherComp :type Primitive%20Component%20Object%20Reference) (OtherBodyIndex :type Integer) (bFromSweep :type Boolean) (SweepResult :type Hit%20Result%20Structure%20%28by%20ref%29))
  (if (!= OtherActor (Components|GetOwner))
    (CallFunction|HandleImpact OtherActor)))

(event EventBeginPlay
  ;[0.15 0.15 0.15 0.5] On spawn, set Projectile to destroy itself after 2 seconds
  (Actor|SetLifeSpan 3.0))

(fn ConstructionScript)

(fn HandleImpact
  (params (OtherActor :type Actor%20Object%20Reference))
  (Game|Damage|ApplyDamage OtherActor (Variables|Default|GetDamage) (Game|GetInstigatorController) self)
  (Actor|DestroyActor))