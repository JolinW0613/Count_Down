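; AI controller for monsters that runs BP_MonsterTree and drives their attacks on the player.
; Perception updates set the blackboard's CanSee flag when the sensed character carries the Faction.Player gameplay tag.
; Tick compares the monster's distance to player 0 against its attack range and calls TryAttack when close enough, with a trait check that inserts a Delay beforehand.
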(event OnTargetPerceptionUpdated(AIPerception)
  (params (Actor :type Actor%20Object%20Reference) (Stimulus :type AI%20Stimulus%20Structure))
  ;[0.15 0.15 0.15 0.5] AI Moving Logic
  (bind _asbp_twin_stick_character (Utilities|Casting|CastToBP_TwinStickCharacter Actor))
  (if (GameplayTags|HasTag (Variables|/Game/BluePrint/BP_TwinStickCharacter.BP_TwinStickCharacter_C|GetGameplayTags _asbp_twin_stick_character) "(TagName=\"Faction.Player\")" true)
    (AI|Components|Blackboard|SetValueasBool (AI|GetBlackboard self) (Utilities|Name|MakeLiteralName "CanSee") (.bSuccessfullySensed (Utilities|Struct|BreakAIStimulus Stimulus)))))

(event EventBeginPlay
  (AI|RunBehaviorTree "/Game/BluePrint/AI/BP_MonsterTree.BP_MonsterTree"))

(event EventTick
  (params (DeltaSeconds :type Float%20%28single-precision%29))
  ;[0.15 0.15 0.15 0.5] Monster Attacking
  (bind _asbp_monster_base (Utilities|Casting|CastToBP_MonsterBase (Pawn|GetControlledPawn)))
  (bind _hastrait (Default|HasTraits _asbp_monster_base "NewEnumerator2"))
  (if _hastrait
    (Utilities|FlowControl|Delay 1.0))
  (bind _range (Default|GetDamageandRange _asbp_monster_base))
  (if (<= (Math|Vector|Distance(Vector) (Transformation|GetActorLocation _asbp_monster_base) (Transformation|GetActorLocation (Game|GetPlayerCharacter 0))) _range)
    (Default|TryAttack _asbp_monster_base (Game|GetPlayerCharacter 0))))

(fn ConstructionScript)