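; Behavior Tree task that wanders an AI pawn to a random reachable point nearby.
; It projects the pawn's location onto the navmesh, picks a random reachable point within a fixed radius and runs AI MoveTo.
; The task finishes with the move's result, or fails with a debug print when either navigation query fails.
; An invalid controller or pawn leaves the task without a FinishExecute call.
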(event EventReceiveExecuteAI
  (params (OwnerController :type AI%20Controller%20Object%20Reference) (ControlledPawn :type Pawn%20Object%20Reference))
  (bind _returnvalue (Transformation|GetActorLocation ControlledPawn))
  (bind (_projectedlocation _returnvalue_2) (AI|Navigation|ProjectPointtoNavigation _returnvalue 0 "/Script/NavigationSystem.NavigationQueryFilter" "200.000000,200.000000,500.000000"))
  (bind (_randomlocation _returnvalue_3) (AI|Navigation|GetRandomReachablePointinRadius _projectedlocation 5e+02 0 "/Script/NavigationSystem.NavigationQueryFilter"))
  (if (Utilities|IsValid ControlledPawn)
    (if (Utilities|IsValid OwnerController)
      (if _returnvalue_2
        (if _returnvalue_3
          (AI|AIMoveTo ControlledPawn _randomlocation 0 5e+01 true
            (:OnSuccess
              (Development|PrintString "RANDOM POINT SUCCESS")
              (AI|BehaviorTree|FinishExecute true))
            (:OnFail
              (AI|BehaviorTree|FinishExecute false :!label _label)))
          (else
            (Development|PrintString "RANDOM POINT FAILED" :!label _label_2)
            (goto _label)))
        (else
          (goto _label_2))))))